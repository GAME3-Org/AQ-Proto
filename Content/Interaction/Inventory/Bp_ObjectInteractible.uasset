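; Bp_ObjectInteractible is an interactible inventory object with pickup functions, apparently still a work in progress.
; PickUpIt prints debug text, fires the Interaggit event and returns the Item variable, while PickUpItem only prints and returns Item.
; PickUp and GetInteractionWidgetRef are empty.
; Destruction is disconnected: PickUpIt never reaches DestroyItem, whose delay leads nowhere, and DestroyActor never runs.
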(event `Destroy Item`
  (`KismetSystemLibrary.Delay` 0.2))

(event `Interaggit`
  (`KismetSystemLibrary.PrintString` "interragit"))

(fn `GetInteractionWidgetRef`
  (returns (RefWidget :type "WidgetComponent Object Reference"))
  (return null))

(fn `PickUp`
  (return))

(fn `PickUpIt`
  (returns (item :type String))
  (bind _item (`self.item`))
  (`KismetSystemLibrary.PrintString` "item picked!")
  (`KismetSystemLibrary.PrintString` _item)
  (`self.Interaggit`)
  (return _item))

(fn `PickUpItem`
  (returns (item :type String))
  (`KismetSystemLibrary.PrintString` "item interragit")
  (return (`self.item`)))

(fn `UserConstructionScript`)